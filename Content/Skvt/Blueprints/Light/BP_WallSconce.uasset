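; BP_WallSconce is a wall sconce light actor with a configurable spotlight that can be switched on or off.
; The construction script applies exposed brightness, color, inner and outer cone angles, and on/off state to SconceLight.
; BeginPlay reapplies the visibility from IsOn, and ToggleLight sets the light's visibility from the value passed in.
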(event `self.ReceiveBeginPlay`
  (`SceneComponent.SetVisibility` (`self.SconceLight`) (`self.IsOn`) false))

(fn `ToggleLight`
  (params (IsOn :type Boolean))
  (`SceneComponent.SetVisibility` (`self.SconceLight`) IsOn false))

(fn `UserConstructionScript`
  (bind _sconcelight (`self.SconceLight`))
  (`LightComponent.SetIntensity` _sconcelight (`self.Brightness`))
  (`LightComponent.SetLightColor` _sconcelight (`self.Color`) true)
  (`SpotLightComponent.SetInnerConeAngle` _sconcelight (`self.Inner Cone Angle`))
  (`SpotLightComponent.SetOuterConeAngle` _sconcelight (`self.Outer Cone Angle`))
  (`SceneComponent.SetVisibility` (`self.SconceLight`) (`self.IsOn`) false))